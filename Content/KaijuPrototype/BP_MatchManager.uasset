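; Match manager actor that runs a round-based brawler fight between the player and one AI enemy per round.
; A 0.2-second looping timer refreshes HUD health bars and checks deaths, starting the next round or ending the match with a win or loss.
; Round state lives in the Colossus GameMode and GameState; each round spawns an enemy at its indexed spawn point, with a health override in round two.
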(event `self.ReceiveBeginPlay`
  (bind _ascolossus_game_state (cast `ColossusGameState` (`GameplayStatics.GetGameState`)))
  (set `self.ColossusGameStateRef` _ascolossus_game_state)
  (bind _ascolossus_game_mode (cast `ColossusGameMode` (`GameplayStatics.GetGameMode`)))
  (set `self.ColossusGameModeRef` _ascolossus_game_mode)
  (bind _asbrawler_character (cast `BrawlerCharacter` (`GameplayStatics.GetPlayerCharacter` 0)))
  (set `self.Player` _asbrawler_character)
  (`KismetSystemLibrary.K2_SetTimerDelegate` (delegate `CheckMatchState`) 0.2 true)
  (bind _returnvalue (`|CreateWidget` "/Game/KaijuPrototype/WBP_MatchHUD.WBP_MatchHUD_C" (`GameplayStatics.GetPlayerController` 0)))
  (bind _output_get (set `self.MatchHUD` _returnvalue))
  (`UserWidget.AddToViewport` _output_get 50)
  (`KismetSystemLibrary.Delay` 1.0)
  (`self.StartRound`))

(event `CheckMatchState`
  (bind _currentenemy (`self.CurrentEnemy`))
  (`self.UpdateHUDHealth`)
  (if (not (`|EnumEquality` (`ColossusGameState.GetRoundPhase` (`self.ColossusGameStateRef`)) "Complete"))
    (`/Engine/EditorBlueprintResources/StandardMacros.IsValid` (`self.Player`)
      (:`Is Valid`
        (if (`BrawlerCharacter.IsAlive` (`self.Player`))
          (`/Engine/EditorBlueprintResources/StandardMacros.IsValid` _currentenemy
            (:`Is Valid`
              (if (not (`BrawlerCharacter.IsAlive` _currentenemy))
                (bind _returnvalue (`ColossusGameMode.BeginBetweenRounds` (`self.ColossusGameModeRef`)))
                (if _returnvalue
                  (`KismetSystemLibrary.Delay` 2.0)
                  (`self.StartRound`)
                  (else
                    (`self.EndMatch` true))))))
          (else
            (`self.EndMatch` false)))))))

(event `StartRound`
  (bind _matchhud (`self.MatchHUD`))
  (bind _colossusgamestateref (`self.ColossusGameStateRef`))
  (bind _returnvalue (`ColossusGameState.GetCurrentRound` _colossusgamestateref))
  (bind _healthcomponent (`BrawlerCharacter.HealthComponent` (`self.CurrentEnemy`)))
  (bind _output (`|GetArrayItem` (`self.EnemySpawnPoints`) (- _returnvalue 1)))
  (`ColossusGameMode.BeginNextRound` (`self.ColossusGameModeRef`))
  (`/Engine/EditorBlueprintResources/StandardMacros.IsValid` _matchhud
    (:`Is Valid`
      (`/Game/KaijuPrototype/WBP_MatchHUD.ShowRound` _matchhud _returnvalue (`ColossusGameState.GetTotalRounds` _colossusgamestateref))
      (`/Engine/EditorBlueprintResources/StandardMacros.IsValid` _output
        (:`Is Valid`
          (bind _returnvalue_2 (`AIBlueprintHelperLibrary.SpawnAIFromClass` (`self.EnemyClass`) null (`self.K2_GetActorLocation` _output) (`self.K2_GetActorRotation` _output) true null))
          (`self.UpdateHUDHealth`)
          (`/Engine/EditorBlueprintResources/StandardMacros.IsValid` (`Pawn.GetController` _returnvalue_2)
            (:`Is Valid`
              (bind _asbrawler_character (cast `BrawlerCharacter` _returnvalue_2))
              (set `self.CurrentEnemy` _asbrawler_character)
              (if (== (`ColossusGameState.GetCurrentRound` (`self.ColossusGameStateRef`)) 2)
                (bind _output_get (set `BrawlerHealthComponent.MaxHealth` 150.0 _healthcomponent))
                (set `BrawlerHealthComponent.CurrentHealth` _output_get _healthcomponent)
                (`self.UpdateHUDHealth`)
                (`ColossusGameMode.ActivateCurrentRound` (`self.ColossusGameModeRef`))
                (else
                  (`ColossusGameMode.ActivateCurrentRound` (`self.ColossusGameModeRef`)))))))))))

(event `EndMatch`
  (params (PlayerWon :type Boolean))
  (bind _matchhud (`self.MatchHUD`))
  (`ColossusGameMode.CompleteMatch` (`self.ColossusGameModeRef`))
  (`/Engine/EditorBlueprintResources/StandardMacros.IsValid` _matchhud
    (:`Is Valid`
      (`KismetSystemLibrary.Delay` 3.87)
      (`/Game/KaijuPrototype/WBP_MatchHUD.ShowMatchResult` _matchhud PlayerWon))))

(fn `UpdateHUDHealth`
  (bind _player (`self.Player`))
  (bind _currentenemy (`self.CurrentEnemy`))
  (bind _healthcomponent (`BrawlerCharacter.HealthComponent` (`self.CurrentEnemy`)))
  (bind _healthcomponent_2 (`BrawlerCharacter.HealthComponent` (`self.Player`)))
  (`/Engine/EditorBlueprintResources/StandardMacros.IsValid` (`self.MatchHUD`)
    (:`Is Valid`
      (`|ExecutionSequence`
        (:`then_0`
          (`/Engine/EditorBlueprintResources/StandardMacros.IsValid` _player
            (:`Is Valid`
              (`/Engine/EditorBlueprintResources/StandardMacros.IsValid` (`self.GetComponentByClass` _player "/Script/KaijuPrototype.BrawlerHealthComponent")
                (:`Is Valid`
                  (`/Game/KaijuPrototype/WBP_MatchHUD.UpdatePlayerHealth` (`self.MatchHUD`) (`KismetMathLibrary.FClamp` (/ (`BrawlerHealthComponent.CurrentHealth` _healthcomponent_2) (`KismetMathLibrary.FMax` (`BrawlerHealthComponent.MaxHealth` _healthcomponent_2) 1.0)))))))))
        (:`then_1`
          (`/Engine/EditorBlueprintResources/StandardMacros.IsValid` _currentenemy
            (:`Is Valid`
              (`/Engine/EditorBlueprintResources/StandardMacros.IsValid` (`self.GetComponentByClass` _currentenemy "/Script/KaijuPrototype.BrawlerHealthComponent")
                (:`Is Valid`
                  (`/Game/KaijuPrototype/WBP_MatchHUD.UpdateEnemyHealth` (`self.MatchHUD`) (`KismetMathLibrary.FClamp` (/ (`BrawlerHealthComponent.CurrentHealth` _healthcomponent) (`KismetMathLibrary.FMax` (`BrawlerHealthComponent.MaxHealth` _healthcomponent) 1.0)))))))))))))

(fn `UserConstructionScript`)